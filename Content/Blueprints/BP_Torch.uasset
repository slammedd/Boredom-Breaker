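; BP_Torch is a torch Blueprint that gives its point light a randomized flicker.
; On BeginPlay it plays the Flicker timeline and uses only its Update pin as a tick.
; Each update eases the light's intensity toward TargetIntensity, scaled by delta time and FlickerSpeed.
; The same update feeds a short random Delay that, on completion, picks a new random TargetIntensity.
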(event `self.ReceiveBeginPlay`
  (`Timeline|Flicker`
    (:`Update`
      (`|ExecutionSequence`
        (:`then_0`
          (`LightComponent.SetIntensity` (`self.PointLight`) (`KismetMathLibrary.Lerp` (`LightComponentBase.Intensity` (`self.PointLight`)) (`self.Target Intensity`) (* (`GameplayStatics.GetWorldDeltaSeconds`) (`self.Flicker Speed`)))))
        (:`then_1`
          (`KismetSystemLibrary.Delay` (`KismetMathLibrary.RandomFloatInRange` 0.05 0.15))
          (set `self.Target Intensity` (`KismetMathLibrary.RandomFloatInRange` 1.0 800.0)))))))

(fn `UserConstructionScript`)