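; BP_Level_Finish_Star is a collectible star that ends the level when the player character overlaps its box.
; On pickup it disables collision, plays a collect sound, spins rapidly and moves the mesh along Z via a timeline.
; It then slows the spin, animates scale with a second timeline, spawns a smoke poof and, as a temporary placeholder, opens a hardcoded test level.
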(event `self.Box.OnComponentBeginOverlap`
  (params (OverlappedComponent :type "PrimitiveComponent Object Reference") (OtherActor :type "Actor Object Reference") (OtherComp :type "PrimitiveComponent Object Reference") (OtherBodyIndex :type Integer) (bFromSweep :type Boolean) (SweepResult :type "HitResult Structure (by ref)"))
  (bind _staticmesh (`self.StaticMesh`))
  (bind (_relativelocation_x _relativelocation_y) (`KismetMathLibrary.BreakVector` (`SceneComponent.RelativeLocation` _staticmesh)))
  (bind _asbp_player_character (cast `/Game/Blueprints/BP_Player_Character` OtherActor))
  (set `self.Player` _asbp_player_character)
  (`PrimitiveComponent.SetCollisionEnabled` (`self.Box`) "NoCollision")
  (set `RotatingMovementComponent.RotationRate` (struct :`Yaw` 3110.0) (`self.RotatingMovement`))
  (`GameplayStatics.PlaySoundAtLocation` "/Game/Audio/SC_Star_Collect.SC_Star_Collect" (`self.K2_GetActorLocation`) (struct) 1.0 1.0 0.0 null null null null)
  (bind (_direction _z) (`Timeline|Timeline` :!via `PlayFromStart`)
    (:`Update`
      (`SceneComponent.K2_SetRelativeLocation` _staticmesh (`KismetMathLibrary.MakeVector` _relativelocation_x _relativelocation_y (.z _z)) false false))
    (:`Finished`
      (`KismetSystemLibrary.Delay` 0.1)
      (set `RotatingMovementComponent.RotationRate` (struct :`Yaw` 910.0) (`self.RotatingMovement`))
      (`KismetSystemLibrary.Delay` 1.0)
      (bind (_direction_2 _scale) (`Timeline|Timeline_0` :!via `PlayFromStart`)
        (:`Update`
          (`SceneComponent.SetRelativeScale3D` (`self.StaticMesh`) _scale))
        (:`Finished`
          (`NiagaraFunctionLibrary.SpawnSystemAtLocation` "/Game/VFX/NS_Small_Smoke_Poof.NS_Small_Smoke_Poof" (`SceneComponent.K2_GetComponentLocation` (`self.StaticMesh`)))
          (`KismetSystemLibrary.PrintString` "Reloading Level (TEMP)" true true (struct :`R` 1.0 :`G` 0.008304 :`A` 1.0))
          (`GameplayStatics.OpenLevel` "LVL_Test"))))))

(fn `UserConstructionScript`)