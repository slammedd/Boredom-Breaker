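; BP_Combo_Switch is a puzzle element with red, green and blue switches that the player triggers by overlapping their colliders.
; At BeginPlay it creates a dynamic material instance for each coloured component.
; A player character overlap sets that colour's Activated flag and plays a timeline driving its material's Emissive parameter.
; The flags are never read or reset here, and the Activate event is empty.
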(event `self.ReceiveBeginPlay`
  (bind _returnvalue (`PrimitiveComponent.CreateDynamicMaterialInstance` (`self.Red`) 0 "/Game/CuteSpace/Materials/Controllers_Red.Controllers_Red" "None"))
  (set `self.Red Mat` _returnvalue)
  (bind _returnvalue_2 (`PrimitiveComponent.CreateDynamicMaterialInstance` (`self.Green`) 0 "/Game/CuteSpace/Materials/Controllers_Green.Controllers_Green" "None"))
  (set `self.Green Mat` _returnvalue_2)
  (bind _returnvalue_3 (`PrimitiveComponent.CreateDynamicMaterialInstance` (`self.Blue`) 0 "/Game/CuteSpace/Materials/Controllers_Blue.Controllers_Blue" "None"))
  (set `self.Blue Mat` _returnvalue_3))

(event `/Game/Blueprints/Puzzle_Elements/BPI_Interactable.Activate`
  (params (`Hit Location` :type "Vector Structure")))

(event `self.Red Collider.OnComponentBeginOverlap`
  (params (OverlappedComponent :type "PrimitiveComponent Object Reference") (OtherActor :type "Actor Object Reference") (OtherComp :type "PrimitiveComponent Object Reference") (OtherBodyIndex :type Integer) (bFromSweep :type Boolean) (SweepResult :type "HitResult Structure (by ref)"))
  (cast `/Game/Blueprints/BP_Player_Character` OtherActor)
  (set `self.Red Activated` true)
  (bind (_direction _emissive) (`Timeline|Red Mat Animation` :!via `PlayFromStart`)
    (:`Update`
      (`MaterialInstanceDynamic.SetScalarParameterValue` (`self.Red Mat`) "Emissive" _emissive))))

(event `self.Green Collider.OnComponentBeginOverlap`
  (params (OverlappedComponent :type "PrimitiveComponent Object Reference") (OtherActor :type "Actor Object Reference") (OtherComp :type "PrimitiveComponent Object Reference") (OtherBodyIndex :type Integer) (bFromSweep :type Boolean) (SweepResult :type "HitResult Structure (by ref)"))
  (cast `/Game/Blueprints/BP_Player_Character` OtherActor)
  (set `self.Green Activated` true)
  (bind (_direction _emissive) (`Timeline|Green Mat Animation` :!via `PlayFromStart`)
    (:`Update`
      (`MaterialInstanceDynamic.SetScalarParameterValue` (`self.Green Mat`) "Emissive" _emissive))))

(event `self.Blue Collider.OnComponentBeginOverlap`
  (params (OverlappedComponent :type "PrimitiveComponent Object Reference") (OtherActor :type "Actor Object Reference") (OtherComp :type "PrimitiveComponent Object Reference") (OtherBodyIndex :type Integer) (bFromSweep :type Boolean) (SweepResult :type "HitResult Structure (by ref)"))
  (cast `/Game/Blueprints/BP_Player_Character` OtherActor)
  (set `self.Blue Activated` true)
  (bind (_direction _emissive) (`Timeline|Blue Mat Animation` :!via `PlayFromStart`)
    (:`Update`
      (`MaterialInstanceDynamic.SetScalarParameterValue` (`self.Blue Mat`) "Emissive" _emissive))))

(fn `UserConstructionScript`)