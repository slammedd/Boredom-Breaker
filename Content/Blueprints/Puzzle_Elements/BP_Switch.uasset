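; BP_Switch is a puzzle switch that toggles a linked moving platform between raised and lowered.
; On BeginPlay it casts its MovingPlatform reference to BP_Moving_Platform_Up and caches it.
; Activate sets an Activated flag, waits briefly, then calls LowerPlatform or RaisePlatform depending on the platform's PlatformRaised state.
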(event `self.ReceiveBeginPlay`
  (bind _asbp_moving_platform (cast `/Game/Blueprints/Puzzle_Elements/BP_Moving_Platform_Up` (`self.Moving Platform`)))
  (set `self.As BP Moving Platform` _asbp_moving_platform))

(event `/Game/Blueprints/Puzzle_Elements/BPI_Interactable.Activate`
  (params (`Hit Location` :type "Vector Structure"))
  (bind _as_bp_moving_platform (`self.As BP Moving Platform`))
  (set `self.Activated` true)
  (`KismetSystemLibrary.Delay` 1.0)
  (if (`/Game/Blueprints/Puzzle_Elements/BP_Moving_Platform_Up.Platform Raised` _as_bp_moving_platform)
    (`/Game/Blueprints/Puzzle_Elements/BP_Moving_Platform_Up.Lower Platform` _as_bp_moving_platform)
    (else
      (`/Game/Blueprints/Puzzle_Elements/BP_Moving_Platform_Up.Raise Platform ` _as_bp_moving_platform))))

(fn `UserConstructionScript`
  (`parent.UserConstructionScript`))