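; BP_Key is a collectible puzzle key that unlocks its referenced chest when the player character overlaps it.
; Pickup disables the box collision, plays a sound and removes the rotating movement, then the Alpha timeline lerps the key above the chest and angles it relative to the chest.
; The Scale timeline then animates key size, using a DoOnce to play unlock sound and smoke and call SpawnPuzzleElement on BP_Chest.
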(event `self.Box.OnComponentBeginOverlap`
  (params (OverlappedComponent :type "PrimitiveComponent Object Reference") (OtherActor :type "Actor Object Reference") (OtherComp :type "PrimitiveComponent Object Reference") (OtherBodyIndex :type Integer) (bFromSweep :type Boolean) (SweepResult :type "HitResult Structure (by ref)"))
  (bind _key (`self.Key`))
  (bind (_returnvalue_roll _returnvalue_pitch _returnvalue_yaw) (`KismetMathLibrary.BreakRotator` (`KismetMathLibrary.FindLookAtRotation` (`self.K2_GetActorLocation` (`self.Chest`)) (`SceneComponent.K2_GetComponentLocation` _key))))
  (cast `/Game/Blueprints/BP_Player_Character` OtherActor)
  (`PrimitiveComponent.SetCollisionEnabled` (`self.Box`) "NoCollision")
  (`GameplayStatics.PlaySoundAtLocation` "/Game/Audio/SC_Key_Collect.SC_Key_Collect" (`self.K2_GetActorLocation`) (struct) 1.0 1.0 0.0 null null null null)
  (`ActorComponent.K2_DestroyComponent` (`self.RotatingMovement`))
  (bind _result (`/Engine/EditorBlueprintResources/StandardMacros.NegateFloat` _returnvalue_pitch)
    (:`  `
      (bind (_direction _alpha _rotation_alpha) (`Timeline|Alpha` :!via `PlayFromStart`)
        (:`Update`
          (`SceneComponent.K2_SetWorldLocation` (`self.Key`) (`KismetMathLibrary.VLerp` (`SceneComponent.K2_GetComponentLocation` (`self.Key`)) (+ (`self.K2_GetActorLocation` (`self.Chest`)) (0.0 0.0 175.0)) _alpha) false false)
          (`SceneComponent.K2_SetWorldRotation` (`self.Key`) (`KismetMathLibrary.RLerp` (`SceneComponent.K2_GetComponentRotation` _key) (`KismetMathLibrary.MakeRotator` _returnvalue_roll (- _result 45.0) _returnvalue_yaw) _rotation_alpha) false false))
        (:`Finished`
          (bind (_direction_2 _scale) (`Timeline|Scale` :!via `PlayFromStart`)
            (:`Update`
              (`SceneComponent.SetRelativeScale3D` (`self.Key`) (`KismetMathLibrary.MakeVector` _scale _scale _scale))
              (`/Engine/EditorBlueprintResources/StandardMacros.DoOnce` false
                (:`Completed`
                  (`GameplayStatics.PlaySoundAtLocation` "/Game/Audio/SC_Chest_Unlock.SC_Chest_Unlock" (`SceneComponent.K2_GetComponentLocation` (`self.Key`)) (struct) 1.0 1.0 0.0 null null null null)
                  (`NiagaraFunctionLibrary.SpawnSystemAtLocation` "/Game/VFX/NS_Big_Smoke_Poof.NS_Big_Smoke_Poof" (`self.K2_GetActorLocation` (`self.Chest`)))
                  (bind _asbp_chest (cast `/Game/Blueprints/Puzzle_Elements/BP_Chest` (`self.Chest`)))
                  (`/Game/Blueprints/Puzzle_Elements/BP_Chest.Spawn Puzzle Element` _asbp_chest))))))))))

(fn `UserConstructionScript`)