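; Destructible crate puzzle element that breaks when activated by a hit.
; Activate spawns an impact effect at the hit location and plays a timeline that stretches the mesh from its cached base scale.
; When the stretch finishes, it plays a break sound and smoke poof, hides the mesh, then destroys the actor after a short delay.
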(event `self.ReceiveBeginPlay`
  (set `self.Base Scale` (`SceneComponent.RelativeScale3D` (`self.StaticMesh`))))

(event `/Game/Blueprints/Puzzle_Elements/BPI_Interactable.Activate`
  (params (`Hit Location` :type "Vector Structure"))
  (bind _returnvalue (`self.K2_GetActorLocation`))
  (bind _base_scale (`self.Base Scale`))
  (`NiagaraFunctionLibrary.SpawnSystemAtLocation` "/Game/VFX/NS_Hit_Impact.NS_Hit_Impact" `Hit Location`)
  (bind (_direction _alpha) (`Timeline|Box Stretch Animation` :!via `PlayFromStart`)
    (:`Update`
      (`SceneComponent.SetRelativeScale3D` (`self.StaticMesh`) (`KismetMathLibrary.VLerp` _base_scale (* _base_scale (`self.Attack Stretch Factor`)) _alpha)))
    (:`Finished`
      (`GameplayStatics.PlaySoundAtLocation` "/Game/Audio/SC_Crate_Break.SC_Crate_Break" _returnvalue (struct) 1.0 1.0 0.0 null null null null)
      (`NiagaraFunctionLibrary.SpawnSystemAtLocation` "/Game/VFX/NS_Big_Smoke_Poof.NS_Big_Smoke_Poof" _returnvalue)
      (`SceneComponent.SetVisibility` (`self.StaticMesh`) false false)
      (`KismetSystemLibrary.Delay` 1.0)
      (`self.K2_DestroyActor`))))

(fn `UserConstructionScript`)