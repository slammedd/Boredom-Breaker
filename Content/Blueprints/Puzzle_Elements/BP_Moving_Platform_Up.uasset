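; BP_Moving_Platform_Up is a puzzle element platform that moves vertically through its RaisePlatform and LowerPlatform events.
; Each event plays a sound at the actor and runs its own timeline to drive the Platform's relative Z, with lowering played in reverse from the end.
; A PlatformRaised flag gates both events, set as raising starts and cleared only when lowering finishes.
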(event `Raise Platform`
  (bind _platform (`self.Platform`))
  (bind (_relativelocation_x _relativelocation_y) (`KismetMathLibrary.BreakVector` (`SceneComponent.RelativeLocation` _platform)))
  (if (not (`self.Platform Raised`))
    (set `self.Platform Raised` true)
    (`GameplayStatics.PlaySoundAtLocation` "/Game/Audio/SC_Moving_Platform.SC_Moving_Platform" (`self.K2_GetActorLocation`) (struct) 1.0 1.0 0.0 null null null null)
    (bind (_direction _z) (`Timeline|Raise Platform Anim` :!via `PlayFromStart`)
      (:`Update`
        (`SceneComponent.K2_SetRelativeLocation` _platform (`KismetMathLibrary.MakeVector` _relativelocation_x _relativelocation_y _z) false false)))))

(event `Lower Platform`
  (bind _platform (`self.Platform`))
  (bind (_relativelocation_x _relativelocation_y) (`KismetMathLibrary.BreakVector` (`SceneComponent.RelativeLocation` _platform)))
  (if (`self.Platform Raised`)
    (`GameplayStatics.PlaySoundAtLocation` "/Game/Audio/SC_Moving_Platform.SC_Moving_Platform" (`self.K2_GetActorLocation`) (struct) 1.0 1.0 0.0 null null null null)
    (bind (_direction _z) (`Timeline|Lower Platform Anim` :!via `ReverseFromEnd`)
      (:`Update`
        (`SceneComponent.K2_SetRelativeLocation` _platform (`KismetMathLibrary.MakeVector` _relativelocation_x _relativelocation_y _z) false false))
      (:`Finished`
        (set `self.Platform Raised` false)))))

(fn `UserConstructionScript`)