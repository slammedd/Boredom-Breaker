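; BP_Door is a puzzle gate that opens and closes through RaiseDoor and LowerDoor events, guarded by an Open flag.
; Separate timelines animate GateHolder's Z scale, with LowerDoor playing its timeline in reverse.
; Both events trigger player screenshake and the same sound, with smoke firing as raising starts and lowering finishes.
; Blocker collision switches off once raised and back on once lowered, when Open also clears.
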(event `Raise Door`
  (bind _gate_holder (`self.Gate Holder`))
  (bind (_relativescale3d_x _relativescale3d_y) (`KismetMathLibrary.BreakVector` (`SceneComponent.RelativeScale3D` _gate_holder)))
  (if (not (`self.Open`))
    (set `self.Open` true)
    (bind _asbp_player_character (cast `/Game/Blueprints/BP_Player_Character` (`GameplayStatics.GetPlayerCharacter` 0)))
    (`/Game/Blueprints/BP_Player_Character.Small Screenshake` _asbp_player_character)
    (`ActorComponent.Activate` (`self.NS_Door_Smoke_R`) false)
    (`ActorComponent.Activate` (`self.NS_Door_Smoke_L`) false)
    (`GameplayStatics.PlaySoundAtLocation` "/Game/Audio/SC_Door_Open.SC_Door_Open" (`self.K2_GetActorLocation`) (struct) 1.0 1.0 0.0 null null null null)
    (bind (_direction _scale) (`Timeline|Raise_Door` :!via `PlayFromStart`)
      (:`Update`
        (`SceneComponent.SetRelativeScale3D` _gate_holder (`KismetMathLibrary.MakeVector` _relativescale3d_x _relativescale3d_y _scale)))
      (:`Finished`
        (`PrimitiveComponent.SetCollisionEnabled` (`self.Blocker`) "NoCollision")))))

(event `Lower Door`
  (bind _gate_holder (`self.Gate Holder`))
  (bind (_relativescale3d_x _relativescale3d_y) (`KismetMathLibrary.BreakVector` (`SceneComponent.RelativeScale3D` _gate_holder)))
  (if (`self.Open`)
    (bind _asbp_player_character (cast `/Game/Blueprints/BP_Player_Character` (`GameplayStatics.GetPlayerCharacter` 0)))
    (`/Game/Blueprints/BP_Player_Character.Small Screenshake` _asbp_player_character)
    (`GameplayStatics.PlaySoundAtLocation` "/Game/Audio/SC_Door_Open.SC_Door_Open" (`self.K2_GetActorLocation`) (struct) 1.0 1.0 0.0 null null null null)
    (bind (_direction _scale) (`Timeline|Timeline` :!via `ReverseFromEnd`)
      (:`Update`
        (`SceneComponent.SetRelativeScale3D` _gate_holder (`KismetMathLibrary.MakeVector` _relativescale3d_x _relativescale3d_y _scale)))
      (:`Finished`
        (set `self.Open` false)
        (`ActorComponent.Activate` (`self.NS_Door_Smoke_R`) false)
        (`ActorComponent.Activate` (`self.NS_Door_Smoke_L`) false)
        (`PrimitiveComponent.SetCollisionEnabled` (`self.Blocker`) "QueryAndPhysics")))))

(fn `UserConstructionScript`)