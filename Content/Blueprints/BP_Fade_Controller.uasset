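; BP_Fade_Controller is a trigger that toggles a dissolve fade each time the player character overlaps its box.
; Depending on the Visible flag, an overlap plays a swoosh sound and runs FadeOut or FadeIn, with CanFade blocking retriggers until the timeline finishes.
; Timelines drive the Dissolve scalar in MPC_Dissolve, a shared material parameter collection.
; Timeline names are crossed: FadeOut plays FadeInAnimation forward, while FadeIn reverses FadeOutAnimation.
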(event `self.Box.OnComponentBeginOverlap`
  (params (OverlappedComponent :type "PrimitiveComponent Object Reference") (OtherActor :type "Actor Object Reference") (OtherComp :type "PrimitiveComponent Object Reference") (OtherBodyIndex :type Integer) (bFromSweep :type Boolean) (SweepResult :type "HitResult Structure (by ref)"))
  (bind _returnvalue (`SceneComponent.K2_GetComponentLocation` (`self.Box`)))
  (cast `/Game/Blueprints/BP_Player_Character` OtherActor)
  (if (`self.Can Fade`)
    (if (`self.Visible`)
      (`GameplayStatics.PlaySoundAtLocation` "/Game/Audio/SC_Swoosh_Deep.SC_Swoosh_Deep" _returnvalue (struct) 1.0 1.0 0.0 null null null null)
      (`self.Fade Out`)
      (else
        (`GameplayStatics.PlaySoundAtLocation` "/Game/Audio/SC_Swoosh_Deep.SC_Swoosh_Deep" _returnvalue (struct) 1.0 1.0 0.0 null null null null)
        (`self.Fade In`)))))

(event `Fade Out`
  (set `self.Can Fade` false)
  (bind (_direction _dissolve) (`Timeline|Fade In Animation` :!via `PlayFromStart`)
    (:`Update`
      (`KismetMaterialLibrary.SetScalarParameterValue` "/Game/Materials/MPC_Dissolve.MPC_Dissolve" "Dissolve" _dissolve))
    (:`Finished`
      (set `self.Can Fade` true)
      (set `self.Visible` false))))

(event `Fade In`
  (set `self.Can Fade` false)
  (bind (_direction _dissolve) (`Timeline|Fade Out Animation` :!via `ReverseFromEnd`)
    (:`Update`
      (`KismetMaterialLibrary.SetScalarParameterValue` "/Game/Materials/MPC_Dissolve.MPC_Dissolve" "Dissolve" _dissolve))
    (:`Finished`
      (set `self.Can Fade` true)
      (set `self.Visible` true))))

(fn `UserConstructionScript`)