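; BP_World2_Menu is a world-space menu Blueprint whose Widget component keeps turning toward the player camera.
; Every Tick, it computes the look-at rotation between the first player's camera and the widget's location.
; It negates the pitch with an added upward tilt offset and flips the yaw half a turn, so the widget faces the camera like a billboard.
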(event `self.ReceiveTick`
  (params (DeltaSeconds :type "Float (single-precision)"))
  (`SceneComponent.K2_SetWorldRotation` (`self.Widget`) (`KismetMathLibrary.MakeRotator` (.roll (`KismetMathLibrary.FindLookAtRotation` (`PlayerCameraManager.GetCameraLocation` (`GameplayStatics.GetPlayerCameraManager` 0)) (`SceneComponent.K2_GetComponentLocation` (`self.Widget`)))) (+ (* (.pitch (`KismetMathLibrary.FindLookAtRotation` (`PlayerCameraManager.GetCameraLocation` (`GameplayStatics.GetPlayerCameraManager` 0)) (`SceneComponent.K2_GetComponentLocation` (`self.Widget`)))) -1.0) 20.0) (+ (.yaw (`KismetMathLibrary.FindLookAtRotation` (`PlayerCameraManager.GetCameraLocation` (`GameplayStatics.GetPlayerCameraManager` 0)) (`SceneComponent.K2_GetComponentLocation` (`self.Widget`)))) 180.0)) false false))

(fn `UserConstructionScript`)